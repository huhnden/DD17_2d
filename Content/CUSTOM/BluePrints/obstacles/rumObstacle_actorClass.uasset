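; Rum obstacle actor for a side-scroller that drifts left at a speed scaled by the game mode's difficulty.
; On spawn it scales itself up, sets its pitch from RandomNumber (its randomizing setter is unwired) and destroys itself after a fixed delay.
; Tick applies a per-frame offset, not scaled by delta time, and plays a sine timeline that wiggles SceneRotate's pitch.
; GetAttachPoint exposes the Arrow's world transform.
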(event EventBeginPlay
  ;[1 1 1] get myDB
  (bind _outactors (Actor|GetAllActorsOfClass "/Game/CUSTOM/BluePrints/myDB.myDB_C"))
  (Variables|Default|SetmyDB_ref (Utilities|Array|Get(acopy) _outactors))
  ;[1 1 1] Set transform of "Scene"
  (Transformation|SetWorldTransform (Variables|Default|GetScene) (Math|Transform|MakeTransform (.Location (Math|Transform|BreakTransform (Transformation|GetWorldTransform (Variables|Default|GetScene)))) (Math|Rotator|MakeRotator 0.0 (Math|Conversions|ToFloat(Integer) (stale _output_get)) 0.0) "4.000000,4.000000,4.000000") false true)
  (Variables|Default|Setobstacle_rotation 1.0)
  ;[1 1 1] Obstacle Movement + game dificulty
  (bind _as2dside_scroller_game_mode (Utilities|Casting|CastTo2DSideScrollerGameMode (Game|GetGameMode)))
  (Variables|Default|Setobstacle_movement (* -2.0 (Variables|/Game/2DSideScrollerBP/Blueprints/2DSideScrollerGameMode.2DSideScrollerGameMode_C|GetgameDificulty _as2dside_scroller_game_mode)))
  (Utilities|FlowControl|Delay 22.0)
  (Actor|DestroyActor))

(event Collision|EventActorBeginOverlap
  (params (OtherActor :type Actor%20Object%20Reference)))

(event EventTick
  (params (DeltaSeconds :type Float%20%28single-precision%29))
  (Variables|Default|SetdeltaTime DeltaSeconds)
  ;[1 1 1] Set "Scene" transform (left movement)
  (Class|SceneComponent|AddWorldTransform (Variables|Default|GetScene) (Math|Transform|MakeTransform (Math|Vector|MakeVector (Variables|Default|Getobstacle_movement) 0.0 0.0) "0, 0, 0" "0.000000,0.000000,0.000000") false true)
  ;[1 1 1] Sinus Wiggle
  (bind _sinus (Timeline|Timeline_0 Play)
    (:Update
      ;[1 1 1] Set "sceneRotate" rotation
      (Transformation|AddLocalRotation (Variables|Default|GetsceneRotate) (Math|Rotator|MakeRotator 0.0 (* _sinus 0.5) 0.0) false true))))

(fn ConstructionScript)

(fn GetAttachPoint
  (return (Transformation|GetWorldTransform (Variables|Default|GetArrow))))