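; Wave obstacle actor that travels along negative world X while spinning around its local pitch axis.
; Each Tick teleports the Scene component a fixed step without sweeping, then adds a local pitch rotation of delta time plus a constant.
; Both motions are frame-rate dependent, and the rotation increment is printed every frame as debug output.
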(event `self.ReceiveTick`
  (params (DeltaSeconds :type "Float (single-precision)"))
  (bind _scene (`self.Scene`))
  (bind _output_get (set `self.obstacle_rotation` (+ DeltaSeconds 1.0)))
  (set `self.obstacle_movement` (+ (.x (.location (`SceneComponent.K2_GetComponentToWorld` (`self.Scene`)))) -3.0))
  (`KismetSystemLibrary.PrintString` (`KismetStringLibrary.Conv_DoubleToString` _output_get))
  (`SceneComponent.K2_SetWorldTransform` _scene (`KismetMathLibrary.MakeTransform` (`KismetMathLibrary.MakeVector` (`self.obstacle_movement`) (.y (.location (`SceneComponent.K2_GetComponentToWorld` (`self.Scene`)))) (.z (.location (`SceneComponent.K2_GetComponentToWorld` (`self.Scene`))))) (.rotation (`SceneComponent.K2_GetComponentToWorld` (`self.Scene`))) (.scale (`SceneComponent.K2_GetComponentToWorld` (`self.Scene`)))) false true)
  (`SceneComponent.K2_AddLocalRotation` _scene (`KismetMathLibrary.MakeRotator` 0.0 (`self.obstacle_rotation`)) false false))

(fn `UserConstructionScript`)