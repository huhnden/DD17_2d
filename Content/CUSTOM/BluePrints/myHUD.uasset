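; myHUD is the HUD Blueprint that puts the score widgets on screen.
; On BeginPlay it caches the MyDB actor and picks a widget by level name: GameOver_score_UI for gameOver, Score_UI for 2DSideScrollerExampleMap.
; Tick polls MyDB's PlayerDeath flag and, while it is true, creates and adds a new GameOver_score_UI every frame, with no guard against duplicates.
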(event `self.ReceiveBeginPlay`
  (bind _outactors (`GameplayStatics.GetAllActorsOfClass` "/Game/CUSTOM/BluePrints/myDB.myDB_C"))
  (set `self.myDB_ref` (`KismetArrayLibrary.Array_Get` _outactors))
  (bind _returnvalue (`GameplayStatics.GetCurrentLevelName` true))
  (if (`KismetStringLibrary.EqualEqual_StrStr` _returnvalue "gameOver")
    (bind _returnvalue_2 (`|CreateWidget` "/Game/CUSTOM/Score/gameOver_score_UI.gameOver_score_UI_C" (`GameplayStatics.GetPlayerController` 0)))
    (`UserWidget.AddToViewport` _returnvalue_2 0)
    (elif (`KismetStringLibrary.EqualEqual_StrStr` _returnvalue "2DSideScrollerExampleMap")
      (bind _returnvalue_3 (`|CreateWidget` "/Game/CUSTOM/Score/score_UI.score_UI_C" (`GameplayStatics.GetPlayerController` 0)))
      (`UserWidget.AddToViewport` _returnvalue_3 0))))

(event `self.ReceiveTick`
  (params (DeltaSeconds :type "Float (single-precision)"))
  (if (`/Game/CUSTOM/BluePrints/myDB.playerDeath` (`self.myDB_ref`))
    (bind _returnvalue (`|CreateWidget` "/Game/CUSTOM/Score/gameOver_score_UI.gameOver_score_UI_C" (`GameplayStatics.GetPlayerController` 0)))
    (`UserWidget.AddToViewport` _returnvalue 0)))

(fn `UserConstructionScript`)